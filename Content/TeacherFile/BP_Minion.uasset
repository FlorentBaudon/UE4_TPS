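; BP_Minion is a player-controlled melee character that moves, turns, attacks, takes damage and dies.
; On begin play it fills health and adds the HUD widget to the viewport.
; Attack starts a montage or queues the alternate section while it plays, and a separate event applies damage through a sphere overlap at the mesh's DamageSocket.
; Incoming damage reduces health, and death disables movement and capsule collision and sets a Dead flag.
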(event Custom|Dead
  (bind _charactermovement (Variables|Character|GetCharacterMovement))
  (Components|Movement|StopMovementImmediately _charactermovement)
  (Pawn|Components|CharacterMovement|DisableMovement _charactermovement)
  (Collision|SetCollisionEnabled (Variables|Collision|GetCapsuleComponent) "NoCollision")
  (Variables|Default|SetbDead true))

(event Custom|ApplyDamage
  (bind _outactors (Collision|SphereOverlapActors (Transformation|GetSocketLocation (Variables|Character|GetMesh) "DamageSocket") 3e+01 (Utilities|Array|MakeArray "ObjectTypeQuery3") 0 (Utilities|Array|MakeArray self)))
  (for _array_element _outactors
    (Game|Damage|ApplyDamage _array_element (Variables|Default|GetDamage) 0 0)))

(event Custom|Attack
  (bind _mesh (Variables|Character|GetMesh))
  (bind _returnvalue (Components|SkeletalMesh|GetAnimInstance _mesh))
  (bind _returnvalue_2 (Animation|Montage|MontageGetCurrentSection _returnvalue "/Game/TeacherFile/Minion_AttackMontage.Minion_AttackMontage"))
  (if (Class|AnimInstance|MontageIsActive _returnvalue "/Game/TeacherFile/Minion_AttackMontage.Minion_AttackMontage")
    (switch name _returnvalue_2
      (:Attack1
        (Class|AnimInstance|MontageSetNextSection _returnvalue _returnvalue_2 "Attack2" "/Game/TeacherFile/Minion_AttackMontage.Minion_AttackMontage"))
      (:Attack2
        (Class|AnimInstance|MontageSetNextSection _returnvalue _returnvalue_2 "Attack1" "/Game/TeacherFile/Minion_AttackMontage.Minion_AttackMontage")))
    (else
      (Animation|PlayAnimMontage "/Game/TeacherFile/Minion_AttackMontage.Minion_AttackMontage" 1.0 "Attack1"))))

(event EventBeginPlay
  (Variables|Default|Sethealth (Variables|Default|GetmaxHealth))
  (bind _returnvalue (UserInterface|CreateWidget "/Game/TeacherFile/WBP_HUD.WBP_HUD_C" (Game|GetPlayerController 0)))
  (UserInterface|Viewport|AddtoViewport _returnvalue 0))

(event Collision|EventActorBeginOverlap
  (params (OtherActor :type Actor%20Object%20Reference)))

(event EventTick
  (params (DeltaSeconds :type Float%20%28single-precision%29)))

(event Game|Damage|EventAnyDamage
  (params (Damage :type Float%20%28single-precision%29) (DamageType :type Damage%20Type%20Object%20Reference) (InstigatedBy :type Controller%20Object%20Reference) (DamageCauser :type Actor%20Object%20Reference))
  (bind _output_get (Variables|Default|Sethealth (- (Variables|Default|Gethealth) Damage)))
  (if (<= _output_get 0.0)
    (CallFunction|Dead)))

(event Input|ActionEvents|InputActionAttack
  (params (Key :type Key%20Structure))
  (:Pressed
    (CallFunction|Attack)))

(event Input|AxisEvents|InputAxisForward
  (params (AxisValue :type Float%20%28single-precision%29))
  (Pawn|Input|AddMovementInput (Math|Vector|GetForwardVector (Transformation|GetActorRotation)) AxisValue false))

(event Input|AxisEvents|InputAxisRight
  (params (AxisValue :type Float%20%28single-precision%29))
  (Pawn|Input|AddMovementInput (Math|Vector|GetRightVector (Transformation|GetActorRotation)) AxisValue false))

(event Input|AxisEvents|InputAxisTurnHorizontal
  (params (AxisValue :type Float%20%28single-precision%29))
  (Pawn|Input|AddControllerYawInput AxisValue))

(event Input|AxisEvents|InputAxisTurnVertical
  (params (AxisValue :type Float%20%28single-precision%29))
  (Pawn|Input|AddControllerPitchInput AxisValue))

(fn ConstructionScript)